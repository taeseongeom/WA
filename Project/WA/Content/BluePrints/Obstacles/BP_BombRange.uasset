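; BP_BombRange is a short-lived damage area obstacle, named as a bomb's blast range.
; On overlap it applies damage to any actor tagged Character, crediting the first player controller as instigator.
; Tick accumulates time and destroys the DamageRange component once LifeSpan is exceeded, while the actor itself expires after three seconds.
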(event `self.ReceiveBeginPlay`
  (`self.SetLifeSpan` 3.0))

(event `self.ReceiveActorBeginOverlap`
  (params (OtherActor :type "Actor Object Reference"))
  (if (`self.ActorHasTag` OtherActor "Character")
    (`GameplayStatics.ApplyDamage` OtherActor (`self.damage`) (`GameplayStatics.GetPlayerController` 0) self "/Script/Engine.DamageType")))

(event `self.ReceiveTick`
  (params (DeltaSeconds :type "Float (single-precision)"))
  (bind _output_get (set `self.timer` (+ DeltaSeconds (`self.timer`))))
  (if (> _output_get (`self.lifeSpan`))
    (`ActorComponent.K2_DestroyComponent` (`self.DamageRange`))))

(fn `UserConstructionScript`)