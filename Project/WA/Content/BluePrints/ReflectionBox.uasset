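; ReflectionBox is an interactable box that the player can hold and move with the Interaction input.
; Overlapping InteractionRegion with a PlayerCharacter-tagged actor enables interaction and caches the PlayerPawn.
; Pressing stores the distance to the player and disables BodyCollider physics; releasing stops movement without restoring physics.
; While held, Tick copies the player's rotation and sets location to forward vector times distance, without adding player location.
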(event `self.ReceiveBeginPlay`)

(event `self.ReceiveTick`
  (params (DeltaSeconds :type "Float (single-precision)"))
  (bind _playeractor (`self.playerActor`))
  (if (`self.move_activate`)
    (`self.K2_SetActorLocationAndRotation` (* (`self.GetActorForwardVector` _playeractor) (`self.distance`)) (`self.K2_GetActorRotation` _playeractor))
    (`KismetSystemLibrary.PrintString` "actor moving")))

(event `self.InteractionRegion.OnComponentBeginOverlap`
  (params (OverlappedComponent :type "PrimitiveComponent Object Reference") (OtherActor :type "Actor Object Reference") (OtherComp :type "PrimitiveComponent Object Reference") (OtherBodyIndex :type Integer) (bFromSweep :type Boolean) (SweepResult :type "HitResult Structure (by ref)"))
  (if (`self.ActorHasTag` OtherActor "PlayerCharacter")
    (set `self.interactable` true)
    (bind _asplayer_pawn (cast `PlayerPawn` OtherActor)
      (:`then`
        (set `self.playerActor` _asplayer_pawn)
        (`KismetSystemLibrary.PrintString` "actor overlaped"))
      (:`CastFailed`
        (`KismetSystemLibrary.PrintString` "Can't find Player Pawn Actor")))))

(event `self.InteractionRegion.OnComponentEndOverlap`
  (params (OverlappedComponent :type "PrimitiveComponent Object Reference") (OtherActor :type "Actor Object Reference") (OtherComp :type "PrimitiveComponent Object Reference") (OtherBodyIndex :type Integer))
  (if (`self.ActorHasTag` OtherActor "PlayerCharacter")
    (set `self.interactable` false)
    (`KismetSystemLibrary.PrintString` "actor leave")))

(event `InputAction|Interaction`
  (params (Key :type "Key Structure"))
  (:`Pressed`
    (`KismetSystemLibrary.PrintString` "Interact with Actor")
    (if (`self.interactable`)
      (set `self.move_activate` true)
      (`KismetSystemLibrary.PrintString` "actor move activated")
      (set `self.distance` (`KismetMathLibrary.Vector_Distance` (`self.K2_GetActorLocation`) (`self.K2_GetActorLocation` (`self.playerActor`))))
      (`PrimitiveComponent.SetSimulatePhysics` (`self.BodyCollider`) false)
      (`KismetSystemLibrary.PrintString` "now actor interacting")))
  (:`Released`
    (if (`self.move_activate`)
      (set `self.move_activate` false)
      (`KismetSystemLibrary.PrintString` "actor interaction ended"))))

(fn `UserConstructionScript`)